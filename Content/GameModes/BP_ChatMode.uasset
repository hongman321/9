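; BP_ChatMode is a chat game mode that hosts a number baseball guessing game with a secret unique three-digit number.
; Client messages are relayed to every BP_Controller via GotBroadcast.
; Inside that per-controller loop, guess commands are stripped of their slash, scored for strikes and balls, and printed.
; An exact match prints a win message and generates a new secret, which is first created on BeginPlay.
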(event Custom|GotMessageFromClient
  (params (Msg :type String))
  (bind _outactors (Actor|GetAllActorsOfClass "/Script/Engine.PlayerController"))
  (for _array_element _outactors
    (bind _asbp_controller (Utilities|Casting|CastToBP_Controller _array_element))
    (Default|GotBroadcast _asbp_controller Msg)
    (bind _returnvalue (Class|MyBlueprintFunctionJudgment|ExtractOnlyGuess Msg))
    (bind _returnvalue_2 (Class|MyBlueprintFunctionJudgment|IsGuessCommand _returnvalue))
    (if _returnvalue_2
      (bind _returnvalue_3 (Class|MyBlueprintFunctionJudgment|RemoveSlashPrefix _returnvalue))
      (Class|MyBlueprintFunctionJudgment|CheckNumber _returnvalue_3)
      (bind _returnvalue_4 (Class|MyBlueprintFunctionJudgment|CountStrikes (Variables|Default|GetBaseballNumber) _returnvalue_3))
      (bind _returnvalue_5 (Class|MyBlueprintFunctionJudgment|CountBalls (Variables|Default|GetBaseballNumber) _returnvalue_3))
      (bind _returnvalue_6 (Class|MyBlueprintFunctionJudgment|GetResultString _returnvalue_4 _returnvalue_5))
      (Development|PrintString _returnvalue_6)
      (if (Utilities|Enum|Equal(Enum) _returnvalue_3 (Variables|Default|GetBaseballNumber))
        (bind _returnvalue_7 (Class|MyBlueprintFunctionJudgment|GetWinMessage Msg))
        (Development|PrintString _returnvalue_7)
        (bind _returnvalue_8 (Class|MyBlueprintFunctionJudgment|GenerateUniqueThreeDigitNumber))
        (Variables|Default|SetBaseballNumber _returnvalue_8)))))

(event EventBeginPlay
  (bind _returnvalue (Class|MyBlueprintFunctionJudgment|GenerateUniqueThreeDigitNumber))
  (Variables|Default|SetBaseballNumber _returnvalue))

(event EventTick
  (params (DeltaSeconds :type Float%20%28single-precision%29)))

(fn ConstructionScript)